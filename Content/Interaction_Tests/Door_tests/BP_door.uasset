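; BP_door is a test door that opens for survivors once enough tasks are completed.
; Overlapping Box1 checks the character's survivor flag, then compares the split-screen game mode's completed-task count against TasksNeededToEnter.
; On success the actor snaps to a fixed rotation and hides its Box component, with no animation or closing logic.
; Killers and early survivors only trigger debug print messages.
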(event `self.Box1.OnComponentBeginOverlap`
  (params (OverlappedComponent :type "PrimitiveComponent Object Reference") (OtherActor :type "Actor Object Reference") (OtherComp :type "PrimitiveComponent Object Reference") (OtherBodyIndex :type Integer) (bFromSweep :type Boolean) (SweepResult :type "HitResult Structure (by ref)"))
  (bind _assplit_screen_game_mode (cast `/Game/GameModes/Split_Screen_gameMode` (`GameplayStatics.GetGameMode`)))
  (bind _asthird_person_character (cast `/Game/ThirdPersonBP/Blueprints/ThirdPersonCharacter` OtherActor))
  (if (`/Game/ThirdPersonBP/Blueprints/ThirdPersonCharacter.IsSurviour?` _asthird_person_character)
    (if (>= (`/Game/GameModes/Split_Screen_gameMode.Current Task completed` _assplit_screen_game_mode) (`self.Tasks Needed To Enter`))
      (`self.K2_SetActorRotation` (struct :`Yaw` 90.0))
      (`SceneComponent.SetVisibility` (`self.Box`) false false)
      (else
        (`KismetSystemLibrary.PrintString` "Door Locked")))
    (else
      (`KismetSystemLibrary.PrintString` "you are the killer "))))

(fn `UserConstructionScript`)